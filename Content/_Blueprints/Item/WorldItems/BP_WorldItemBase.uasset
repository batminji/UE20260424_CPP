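; Base actor for items placed in the world, holding ID, serial number, type, name, UI prefix and mesh set through two init functions.
; On BeginPlay it traces downward for one object type and moves itself to the impact point, without checking for a hit.
; Box overlaps with Player-tagged actors fire begin/end dispatchers with itself and toggle the mesh's custom depth rendering as an outline highlight.
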(event `self.ReceiveBeginPlay`
  (`parent.ReceiveBeginPlay`)
  (`self.SnapToLand`))

(event `self.Box.OnComponentBeginOverlap`
  (params (OverlappedComponent :type "PrimitiveComponent Object Reference") (OtherActor :type "Actor Object Reference") (OtherComp :type "PrimitiveComponent Object Reference") (OtherBodyIndex :type Integer) (bFromSweep :type Boolean) (SweepResult :type "HitResult Structure (by ref)"))
  (if (`self.ActorHasTag` OtherActor "Player")
    (`self.OnBeginOverlap` self)
    (`self.EnableOutLine` true)))

(event `self.Box.OnComponentEndOverlap`
  (params (OverlappedComponent :type "PrimitiveComponent Object Reference") (OtherActor :type "Actor Object Reference") (OtherComp :type "PrimitiveComponent Object Reference") (OtherBodyIndex :type Integer))
  (if (`self.ActorHasTag` OtherActor "Player")
    (`self.OnEndOverlap` self)
    (`self.EnableOutLine` false)))

(fn `EnableOutLine`
  (params (bIsEnable :type Boolean))
  (`PrimitiveComponent.SetRenderCustomDepth` (`self.StaticMesh`) bIsEnable))

(fn `Init`
  (params (InID :type Name) (InSerialNumber :type String))
  (set `self.ID` InID)
  (set `self.SerialNumber` InSerialNumber))

(fn `InitWorldItemBaseData`
  (params (InItemType :type "/Game/_Blueprints/Data/Enum/Item/E_ItemType Enum" :default "NewEnumerator0") (InItemName :type Text) (InUIPrefix :type "/Game/_Blueprints/Data/Enum/Item/E_UIPrefix Enum" :default "NewEnumerator0") (InStaticMesh :type "StaticMesh Object Reference"))
  (set `self.ItemType` InItemType)
  (set `self.ItemName` InItemName)
  (set `self.E_UIPrefix` InUIPrefix)
  (`StaticMeshComponent.SetStaticMesh` (`self.StaticMesh`) InStaticMesh))

(fn `SnapToLand`
  (bind _returnvalue (`self.K2_GetActorLocation`))
  (bind _outhit (`KismetSystemLibrary.LineTraceSingleForObjects` _returnvalue (- _returnvalue (0.0 0.0 1000.0)) (`|MakeArray` "ObjectTypeQuery7" :!type "EObjectTypeQuery Enum")))
  (`self.K2_SetActorLocation` (`.ImpactPoint` (`GameplayStatics.BreakHitResult` _outhit))))

(fn `UserConstructionScript`
  (`parent.UserConstructionScript`))