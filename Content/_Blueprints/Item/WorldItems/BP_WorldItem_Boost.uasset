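; BP_WorldItem_Boost is the world item Blueprint for Boost-type items, specializing a parent world item class.
; Init runs the parent setup, then looks up its ID in DT_WorldItem_Boost to pass type, name, UI prefix and static mesh to InitWorldItemBaseData and store the unit weight.
; GetWeight returns that unit weight multiplied by Amount.
; The event graph and construction script add no logic of their own.
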(fn `GetWeight`
  (returns (OutWeight :type Integer))
  (return (* (`self.SingleWeight`) (`self.Amount`))))

(fn `Init`
  (params (InID :type Name) (InSerialNumber :type String))
  (`parent.Init` InID InSerialNumber)
  (bind _returnvalue (`|GetDataTableRow` "/Game/_Blueprints/Data/DataTable/Item/DT_WorldItem_Boost.DT_WorldItem_Boost" (`self.ID`))
    (:`then`
      (`self.InitWorldItemBaseData` (break `/Game/_Blueprints/Data/Struct/Item/S_WorldItem_Useable` _returnvalue) (`.ItemName_6_2135206648146DA209C398A6CAD30746` (break `/Game/_Blueprints/Data/Struct/Item/S_WorldItem_Useable` _returnvalue)) (`.UIPrefix_9_C4D25A224BB226E362574193419BB884` (break `/Game/_Blueprints/Data/Struct/Item/S_WorldItem_Useable` _returnvalue)) (`.StaticMesh_26_A8628D9648AD2CBB077B2FB42A6B048D` (break `/Game/_Blueprints/Data/Struct/Item/S_WorldItem_Useable` _returnvalue)))
      (set `self.SingleWeight` (`.Weight_27_03C3D81E41F3BEAE96C5528D93209F50` (break `/Game/_Blueprints/Data/Struct/Item/S_WorldItem_Useable` _returnvalue))))))

(fn `UserConstructionScript`
  (`parent.UserConstructionScript`))